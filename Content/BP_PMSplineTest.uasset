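; BP_PMSplineTest is a spline actor that links itself to touching splines of the same class, forming a directional path network.
; Its construction script compares both endpoints against every other instance's endpoints within a small tolerance.
; A matched neighbour becomes up or down if its endpoints share world X, otherwise left or right, with the touching end picking which.
; These references fill a two-entry Splines array, one per endpoint; a disconnected branch clears them.
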(fn ConstructionScript
  (bind _splinecomponent (Variables|Default|GetSplineComponent))
  (bind _splines (Variables|Default|GetSplines))
  (bind _returnvalue (Spline|GetLocationatSplinePoint _splinecomponent 0 "World"))
  (bind _returnvalue_2 (Spline|GetLocationatSplinePoint _splinecomponent 1 "World"))
  ;[1 1 1] Setting splines references
  (bind _outactors (Actor|GetAllActorsOfClass "BP_PMSplineTest_C"))
  (for _array_element _outactors
    (if (!= self _array_element)
      (bind _output_get (LocalVariables|SetCheckedSpline _array_element))
      (Utilities|FlowControl|Sequence
        (:then_0
          ;;[1 1 1] index: 0, 0
          (if (Utilities|Operators|EqualEqual _returnvalue (Spline|GetLocationatSplinePoint (Variables|/Script/PacMan.PMSpline|GetSplineComponent _output_get) 0 "World") 2.0)
            (if (Math|Float|NearlyEqual(Float) (.x (Spline|GetLocationatSplinePoint (Variables|/Script/PacMan.PMSpline|GetSplineComponent (LocalVariables|GetCheckedSpline)) 0 "World")) (.x (Spline|GetLocationatSplinePoint (Variables|/Script/PacMan.PMSpline|GetSplineComponent (LocalVariables|GetCheckedSpline)) 1 "World")) 2.0)
              (LocalVariables|SetUP_0 (LocalVariables|GetCheckedSpline))
              (else
                (LocalVariables|SetRIGHT_0 (LocalVariables|GetCheckedSpline))))))
        (:then_1
          ;;[1 1 1] index: 0, 1
          (if (Utilities|Operators|EqualEqual _returnvalue (Spline|GetLocationatSplinePoint (Variables|/Script/PacMan.PMSpline|GetSplineComponent _output_get) 1 "World") 2.0)
            (if (Math|Float|NearlyEqual(Float) (.x (Spline|GetLocationatSplinePoint (Variables|/Script/PacMan.PMSpline|GetSplineComponent (LocalVariables|GetCheckedSpline)) 0 "World")) (.x (Spline|GetLocationatSplinePoint (Variables|/Script/PacMan.PMSpline|GetSplineComponent (LocalVariables|GetCheckedSpline)) 1 "World")) 2.0)
              (LocalVariables|SetDOWN_0 (LocalVariables|GetCheckedSpline))
              (else
                (LocalVariables|SetLEFT_0 (LocalVariables|GetCheckedSpline))))))
        (:then_2
          ;;[1 1 1] index: 1, 0
          (if (Utilities|Operators|EqualEqual _returnvalue_2 (Spline|GetLocationatSplinePoint (Variables|/Script/PacMan.PMSpline|GetSplineComponent _output_get) 0 "World") 2.0)
            (if (Math|Float|NearlyEqual(Float) (.x (Spline|GetLocationatSplinePoint (Variables|/Script/PacMan.PMSpline|GetSplineComponent (LocalVariables|GetCheckedSpline)) 0 "World")) (.x (Spline|GetLocationatSplinePoint (Variables|/Script/PacMan.PMSpline|GetSplineComponent (LocalVariables|GetCheckedSpline)) 1 "World")) 2.0)
              (LocalVariables|SetUP_1 (LocalVariables|GetCheckedSpline))
              (else
                (LocalVariables|SetRIGHT_1 (LocalVariables|GetCheckedSpline))))))
        (:then_3
          ;;[1 1 1] index: 1, 1
          (if (Utilities|Operators|EqualEqual _returnvalue_2 (Spline|GetLocationatSplinePoint (Variables|/Script/PacMan.PMSpline|GetSplineComponent _output_get) 1 "World") 2.0)
            (if (Math|Float|NearlyEqual(Float) (.x (Spline|GetLocationatSplinePoint (Variables|/Script/PacMan.PMSpline|GetSplineComponent (LocalVariables|GetCheckedSpline)) 0 "World")) (.x (Spline|GetLocationatSplinePoint (Variables|/Script/PacMan.PMSpline|GetSplineComponent (LocalVariables|GetCheckedSpline)) 1 "World")) 2.0)
              (LocalVariables|SetDOWN_1 (LocalVariables|GetCheckedSpline))
              (else
                (LocalVariables|SetLEFT_1 (LocalVariables|GetCheckedSpline)))))))))
  (|SetBy-RefVar (Utilities|Array|Get(acopy) _splines) (Utilities|Struct|MakeSplines (LocalVariables|GetUP_0) (LocalVariables|GetDOWN_0) (LocalVariables|GetLEFT_0) (LocalVariables|GetRIGHT_0)))
  (|SetBy-RefVar (Utilities|Array|Get(acopy) _splines 1) (Utilities|Struct|MakeSplines (LocalVariables|GetUP_1) (LocalVariables|GetDOWN_1) (LocalVariables|GetLEFT_1) (LocalVariables|GetRIGHT_1))))