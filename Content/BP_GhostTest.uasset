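; Test ghost actor meant to travel along BP_PMSpline paths, starting on a spline tagged "ghostStart" found at BeginPlay.
; Tick sets its location by spline distance, but multiplies that distance by delta time instead of adding, so it shrinks toward zero.
; CheckIfAtPoint detects arrival at either of the first two spline points, setting the same SplineIndex for both.
; Arrival triggers nothing yet, and Choose New Spline is an empty stub.
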(event EventBeginPlay
  (bind _outactors (Actor|GetAllActorsOfClasswithTag "/Game/BP_PMSpline.BP_PMSpline_C" "ghostStart"))
  (for _array_element _outactors
    (bind _asbp_pmspline (Utilities|Casting|CastToBP_PMSpline _array_element))
    (Utilities|IsValid _asbp_pmspline
      (:Is%20Valid
        (Variables|Default|SetSpline _asbp_pmspline)
        (Variables|Default|SetPositionOnSpline 1.0)
        (Variables|Default|SetMovingDirection 1.0)))))

(event EventTick
  (params (DeltaSeconds :type Float%20%28single-precision%29))
  (bind _output_get (Variables|Default|SetPositionOnSpline (* (* DeltaSeconds (Variables|Default|GetPositionOnSpline)) (Variables|Default|GetMovingDirection))))
  (Transformation|SetActorLocation (Spline|GetLocationatDistanceAlongSpline (Variables|/Script/PacMan.PMSpline|GetSplineComponent (Variables|Default|GetSpline)) _output_get "World") false false)
  (bind _returnvalue (CallFunction|CheckifatPoint))
  (if _returnvalue
    _))

(fn ConstructionScript)

(fn CheckifatPoint
  (if (Utilities|Operators|EqualEqual (Transformation|GetActorLocation) (Spline|GetLocationatSplinePoint (Variables|/Script/PacMan.PMSpline|GetSplineComponent (Variables|Default|GetSpline)) 1 "World") 0.5)
    (Variables|Default|SetSplineIndex 1)
    (return true)
    (elif (Utilities|Operators|EqualEqual (Transformation|GetActorLocation) (Spline|GetLocationatSplinePoint (Variables|/Script/PacMan.PMSpline|GetSplineComponent (Variables|Default|GetSpline)) 0 "World") 0.5)
      (Variables|Default|SetSplineIndex 1)
      (return true)
      (else
        (return false)))))

(fn ChooseNewSpline)