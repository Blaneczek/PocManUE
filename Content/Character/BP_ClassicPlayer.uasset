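; BP_ClassicPlayer is a player character Blueprint that animates its Top and Bottom components in an endless open-and-close, chomping motion.
; BeginPlay calls the parent, then starts two parallel loops that pitch the halves 60 degrees in opposite directions and back.
; Each half uses a pair of timelines driving a rotation Lerp, with each timeline restarting the other on finish, so no Tick logic is needed.
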(event EventBeginPlay
  (|CallParentFunction)
  (Utilities|FlowControl|Sequence
    (:then_0
      (bind _rotation (Timeline|Timeline Play)
        (:Update
          (Transformation|SetRelativeRotation (Variables|Default|GetTop) (Math|Rotator|MakeRotator 0.0 (Math|Float|Lerp 0.0 -6e+01 _rotation) 0.0) false false))
        (:Finished
          (bind _rotation_2 (Timeline|Timeline_1 PlayFromStart)
            (:Update
              (Transformation|SetRelativeRotation (Variables|Default|GetTop) (Math|Rotator|MakeRotator 0.0 (Math|Float|Lerp -6e+01 0.0 _rotation_2) 0.0) false false))
            (:Finished
              (Timeline|Timeline PlayFromStart))))))
    (:then_1
      (bind _rotation_3 (Timeline|Timeline_0 Play)
        (:Update
          (Transformation|SetRelativeRotation (Variables|Default|GetBottom) (Math|Rotator|MakeRotator 0.0 (Math|Float|Lerp 0.0 6e+01 _rotation_3) 0.0) false false))
        (:Finished
          (bind _rotation_4 (Timeline|Timeline_2 PlayFromStart)
            (:Update
              (Transformation|SetRelativeRotation (Variables|Default|GetBottom) (Math|Rotator|MakeRotator 0.0 (Math|Float|Lerp 6e+01 0.0 _rotation_4) 0.0) false false))
            (:Finished
              (Timeline|Timeline_0 PlayFromStart))))))))

(fn ConstructionScript)