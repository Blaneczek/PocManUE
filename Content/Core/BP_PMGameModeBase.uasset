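; Game mode Blueprint for a game with ghosts and cherry coins, meant to manage HUD and end-of-game screens.
; Live events show a starting timer widget and open the Menu level; OnRestartGame is empty.
; Score, cherry and lives widget setup and updates follow parent calls, and won/lost screens bind menu and restart events.
; Those HUD and end-screen chains have no connected entry event, so they never run as shown.
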(event Custom|GoToMenu
  (Game|OpenLevel(byName) "Menu"))

(event Custom|OnRestartGame)

(event EventStartingTimer
  (params (time :type Float%20%28single-precision%29))
  (bind _returnvalue (UserInterface|CreateWidget "/Game/UI/WBP_StartingTimer.WBP_StartingTimer_C"))
  (UserInterface|Viewport|AddtoViewport _returnvalue 0))

(fn ConstructionScript)