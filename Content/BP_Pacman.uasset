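; Pac-Man player actor that travels a maze built from linked BP_Spline segments, starting on the one tagged "Start".
; WASD reverses instantly along the current axis or queues a perpendicular turn as DesiredDirection.
; Tick advances distance along the spline, halts at either endpoint, then switches to the queued or straight-ahead neighbor.
; Neighbor lookups read only SplinesAt0, FindNearestPoint is never called here, and Tick prints CurrentDirection for debugging.
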(event EventBeginPlay
  (bind _outactors (Actor|GetAllActorsOfClasswithTag "/Game/BP_Spline.BP_Spline_C" "Start"))
  (for _array_element _outactors
    (Variables|Default|SetCurrentSpline _array_element)
    (Variables|Default|SetDesiredDirection "NewEnumerator0")
    (Variables|Default|SetDirection 1.0)
    (Variables|Default|SetPosition%20on%20Spline 2.0)
    (Variables|Default|SetCurrentDirection "NewEnumerator1")))

(event EventTick
  (params (DeltaSeconds :type Float%20%28single-precision%29))
  (Development|PrintString (Utilities|String|EnumtoString (Variables|Default|GetCurrentDirection)))
  (Utilities|FlowControl|Sequence
    (:then_0
      (if (Variables|Default|GetbIsMoving)
        (bind _output_get (Variables|Default|SetPosition%20on%20Spline (+ (* (* DeltaSeconds (Variables|Default|GetDirection)) 3e+02) (Variables|Default|GetPosition%20on%20Spline))))
        (Transformation|SetActorLocation (Spline|GetLocationatDistanceAlongSpline (Variables|/Game/BP_Spline.BP_Spline_C|GetSpline (Variables|Default|GetCurrentSpline)) _output_get "World") false false)
        (bind (_returnvalue _index) (CallFunction|CheckifatPoint))
        (if _returnvalue
          (Variables|Default|SetbIsMoving false)
          (Variables|Default|SetSplinesIndex _index))
        (else
          (switch Utilities|FlowControl|Switch|SwitchonEDirections (Variables|Default|GetDesiredDirection)
            (:NewEnumerator0
              (switch Utilities|FlowControl|Switch|SwitchonEDirections (Variables|Default|GetCurrentDirection)
                (:NewEnumerator1
                  (switch int (Variables|Default|GetSplinesIndex)
                    (:0
                      (Utilities|IsValid (.up (Variables|/Game/BP_Spline.BP_Spline_C|GetSplinesAt0 (Variables|Default|GetCurrentSpline)))
                        (:Is%20Valid
                          (Variables|Default|SetCurrentSpline (.up (Variables|/Game/BP_Spline.BP_Spline_C|GetSplinesAt0 (Variables|Default|GetCurrentSpline))))
                          (Variables|Default|SetPosition%20on%20Spline 0.0)
                          (Variables|Default|SetbIsMoving true))))))
                (:NewEnumerator2
                  (Utilities|IsValid (.down (Variables|/Game/BP_Spline.BP_Spline_C|GetSplinesAt0 (Variables|Default|GetCurrentSpline)))
                    (:Is%20Valid
                      (bind _output_get_2 (Variables|Default|SetCurrentSpline (.down (Variables|/Game/BP_Spline.BP_Spline_C|GetSplinesAt0 (Variables|Default|GetCurrentSpline)))))
                      (Variables|Default|SetPosition%20on%20Spline (Spline|GetDistanceAlongSplineatSplinePoint (Variables|/Game/BP_Spline.BP_Spline_C|GetSpline _output_get_2) 1))
                      (Variables|Default|SetbIsMoving true))))
                (:NewEnumerator3
                  (Utilities|IsValid (.left (Variables|/Game/BP_Spline.BP_Spline_C|GetSplinesAt0 (Variables|Default|GetCurrentSpline)))
                    (:Is%20Valid
                      (bind _output_get_3 (Variables|Default|SetCurrentSpline (.left (Variables|/Game/BP_Spline.BP_Spline_C|GetSplinesAt0 (Variables|Default|GetCurrentSpline)))))
                      (Variables|Default|SetPosition%20on%20Spline (Spline|GetDistanceAlongSplineatSplinePoint (Variables|/Game/BP_Spline.BP_Spline_C|GetSpline _output_get_3) 1))
                      (Variables|Default|SetbIsMoving true))))
                (:NewEnumerator4
                  (Utilities|IsValid (.right (Variables|/Game/BP_Spline.BP_Spline_C|GetSplinesAt0 (Variables|Default|GetCurrentSpline)))
                    (:Is%20Valid
                      (Variables|Default|SetCurrentSpline (.right (Variables|/Game/BP_Spline.BP_Spline_C|GetSplinesAt0 (Variables|Default|GetCurrentSpline))))
                      (Variables|Default|SetPosition%20on%20Spline 0.0)
                      (Variables|Default|SetbIsMoving true))))))
            (:NewEnumerator1
              (Utilities|IsValid (.up (Variables|/Game/BP_Spline.BP_Spline_C|GetSplinesAt0 (Variables|Default|GetCurrentSpline)))
                (:Is%20Valid
                  (Variables|Default|SetCurrentSpline (.up (Variables|/Game/BP_Spline.BP_Spline_C|GetSplinesAt0 (Variables|Default|GetCurrentSpline))))
                  (Variables|Default|SetPosition%20on%20Spline 0.0)
                  (Variables|Default|SetDirection 1.0)
                  (Variables|Default|SetDesiredDirection "NewEnumerator0")
                  (Variables|Default|SetCurrentDirection "NewEnumerator1")
                  (Transformation|SetActorRotation "0, 0, 0")
                  (Variables|Default|SetbIsMoving true))))
            (:NewEnumerator2
              (Utilities|IsValid (.down (Variables|/Game/BP_Spline.BP_Spline_C|GetSplinesAt0 (Variables|Default|GetCurrentSpline)))
                (:Is%20Valid
                  (bind _output_get_4 (Variables|Default|SetCurrentSpline (.down (Variables|/Game/BP_Spline.BP_Spline_C|GetSplinesAt0 (Variables|Default|GetCurrentSpline)))))
                  (Variables|Default|SetPosition%20on%20Spline (Spline|GetDistanceAlongSplineatSplinePoint (Variables|/Game/BP_Spline.BP_Spline_C|GetSpline _output_get_4) 1))
                  (Variables|Default|SetDirection -1.0)
                  (Variables|Default|SetDesiredDirection "NewEnumerator0")
                  (Variables|Default|SetCurrentDirection "NewEnumerator2")
                  (Transformation|SetActorRotation "0.000000,180.000000,0.000000")
                  (Variables|Default|SetbIsMoving true))))
            (:NewEnumerator3
              (Utilities|IsValid (.left (Variables|/Game/BP_Spline.BP_Spline_C|GetSplinesAt0 (Variables|Default|GetCurrentSpline)))
                (:Is%20Valid
                  (bind _output_get_5 (Variables|Default|SetCurrentSpline (.left (Variables|/Game/BP_Spline.BP_Spline_C|GetSplinesAt0 (Variables|Default|GetCurrentSpline)))))
                  (Variables|Default|SetPosition%20on%20Spline (Spline|GetDistanceAlongSplineatSplinePoint (Variables|/Game/BP_Spline.BP_Spline_C|GetSpline _output_get_5) 1))
                  (Variables|Default|SetDirection -1.0)
                  (Variables|Default|SetDesiredDirection "NewEnumerator0")
                  (Variables|Default|SetCurrentDirection "NewEnumerator3")
                  (Transformation|SetActorRotation "0.000000,-90.000000,0.000000")
                  (Variables|Default|SetbIsMoving true))))
            (:NewEnumerator4
              (Utilities|IsValid (.right (Variables|/Game/BP_Spline.BP_Spline_C|GetSplinesAt0 (Variables|Default|GetCurrentSpline)))
                (:Is%20Valid
                  (Variables|Default|SetCurrentSpline (.right (Variables|/Game/BP_Spline.BP_Spline_C|GetSplinesAt0 (Variables|Default|GetCurrentSpline))))
                  (Variables|Default|SetPosition%20on%20Spline 0.0)
                  (Variables|Default|SetDirection 1.0)
                  (Variables|Default|SetDesiredDirection "NewEnumerator0")
                  (Variables|Default|SetCurrentDirection "NewEnumerator4")
                  (Transformation|SetActorRotation "0.000000,90.000000,0.000000")
                  (Variables|Default|SetbIsMoving true))))))))))

(event Input|KeyboardEvents|W
  (params (Key :type Key%20Structure :default "None"))
  (:Pressed
    (switch Utilities|FlowControl|Switch|SwitchonEDirections (Variables|Default|GetCurrentDirection)
      (:NewEnumerator2
        (Variables|Default|SetCurrentDirection "NewEnumerator1")
        (Variables|Default|SetDirection 1.0)
        (Transformation|SetActorRotation "0, 0, 0")
        (Variables|Default|SetbIsMoving true))
      (:NewEnumerator3
        (Variables|Default|SetDesiredDirection "NewEnumerator1" :!label _label)
        (Variables|Default|SetbIsMoving true))
      (:NewEnumerator4
        (goto _label)))))

(event Input|KeyboardEvents|S
  (params (Key :type Key%20Structure :default "None"))
  (:Pressed
    (switch Utilities|FlowControl|Switch|SwitchonEDirections (Variables|Default|GetCurrentDirection)
      (:NewEnumerator1
        (Variables|Default|SetCurrentDirection "NewEnumerator2")
        (Variables|Default|SetDirection -1.0)
        (Transformation|SetActorRotation "0.000000,180.000000,0.000000")
        (Variables|Default|SetbIsMoving true))
      (:NewEnumerator3
        (Variables|Default|SetDesiredDirection "NewEnumerator2" :!label _label)
        (Variables|Default|SetbIsMoving true))
      (:NewEnumerator4
        (goto _label)))))

(event Input|KeyboardEvents|D
  (params (Key :type Key%20Structure :default "None"))
  (:Pressed
    (switch Utilities|FlowControl|Switch|SwitchonEDirections (Variables|Default|GetCurrentDirection)
      (:NewEnumerator1
        (Variables|Default|SetDesiredDirection "NewEnumerator4" :!label _label)
        (Variables|Default|SetbIsMoving true))
      (:NewEnumerator2
        (goto _label))
      (:NewEnumerator3
        (Variables|Default|SetCurrentDirection "NewEnumerator4")
        (Variables|Default|SetDirection 1.0)
        (Transformation|SetActorRotation "0.000000,90.000000,0.000000")
        (Variables|Default|SetbIsMoving true)))))

(event Input|KeyboardEvents|A
  (params (Key :type Key%20Structure :default "None"))
  (:Pressed
    (switch Utilities|FlowControl|Switch|SwitchonEDirections (Variables|Default|GetCurrentDirection)
      (:NewEnumerator1
        (Variables|Default|SetDesiredDirection "NewEnumerator3" :!label _label)
        (Variables|Default|SetbIsMoving true))
      (:NewEnumerator2
        (goto _label))
      (:NewEnumerator4
        (Variables|Default|SetCurrentDirection "NewEnumerator3")
        (Variables|Default|SetDirection -1.0)
        (Transformation|SetActorRotation "0.000000,-90.000000,0.000000")
        (Variables|Default|SetbIsMoving true)))))

(fn ConstructionScript)

(fn FindNearestPoint
  (bind _returnvalue (Transformation|GetActorLocation))
  (bind _currentspline (Variables|Default|GetCurrentSpline))
  (bind _spline (Variables|/Game/BP_Spline.BP_Spline_C|GetSpline _currentspline))
  (bind _returnvalue_2 (Class|SplineComponent|FindInputKeyClosesttoWorldLocation _spline _returnvalue))
  (bind _returnvalue_3 (Class|SplineComponent|GetDistanceAlongSplineatSplineInputKey _spline _returnvalue_2))
  (if (> _returnvalue_3 1.0)
    (Variables|Default|SetPosition%20on%20Spline (+ _returnvalue_3 -1.0))
    (Variables|Default|SetDirection -1.0)
    (else
      (Variables|Default|SetPosition%20on%20Spline (+ _returnvalue_3 1.0))
      (Variables|Default|SetDirection 1.0))))

(fn CheckifatPoint
  (bind _returnvalue (Transformation|GetActorLocation))
  (bind _currentspline (Variables|Default|GetCurrentSpline))
  (bind _spline (Variables|/Game/BP_Spline.BP_Spline_C|GetSpline _currentspline))
  (if (Utilities|Operators|EqualEqual _returnvalue (Spline|GetLocationatSplinePoint _spline 0 "World") 0.0)
    (return true 0)
    (elif (Utilities|Operators|EqualEqual _returnvalue (Spline|GetLocationatSplinePoint _spline 1 "World") 0.0)
      (return true 1)
      (else
        (return false 0)))))